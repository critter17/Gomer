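; Hub world NPC that registers itself with the game instance and handles the player's proximity for control prompts and dialogue.
; Box overlap shows the control prompt, guessing keyboard or gamepad from whether WASD is held.
; Leaving hides it and, if talk is unfinished, closes and resets the character's dialogue widget after a delay.
; Also carries dash, wall-check and bounce movement helpers, none called in this graph.
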(event OnComponentBeginOverlap(Box)
  (params (OverlappedComponent :type Primitive%20Component%20Object%20Reference) (OtherActor :type Actor%20Object%20Reference) (OtherComp :type Primitive%20Component%20Object%20Reference) (OtherBodyIndex :type Integer) (bFromSweep :type Boolean) (SweepResult :type Hit%20Result%20Structure%20%28by%20ref%29))
  (bind _returnvalue (Game|GetPlayerController 0))
  (if (== (Utilities|GetClass OtherActor) "/Game/GomerContent/Blueprints/BP_GomerCharacter.BP_GomerCharacter_C")
    (bind _asbp_gomer_character (Utilities|Casting|CastToBP_GomerCharacter OtherActor))
    (bind _output_get (Variables|Default|SetGame%20Instance (Variables|/Game/GomerContent/Blueprints/BP_GomerCharacter.BP_GomerCharacter_C|GetGame%20Instance _asbp_gomer_character)))
    (Variables|/Game/GomerContent/Blueprints/BP_GameInstance.BP_GameInstance_C|SetbControlVisible _output_get true)
    (if (Math|Boolean|ORBoolean (Game|Player|IsInputKeyDown _returnvalue "W") (Game|Player|IsInputKeyDown _returnvalue "S") (Game|Player|IsInputKeyDown _returnvalue "D") (Game|Player|IsInputKeyDown _returnvalue "A"))
      (Variables|/Game/GomerContent/Blueprints/BP_GameInstance.BP_GameInstance_C|SetbGamepad (Variables|Default|GetGame%20Instance) false)
      (else
        (Variables|/Game/GomerContent/Blueprints/BP_GameInstance.BP_GameInstance_C|SetbGamepad (Variables|Default|GetGame%20Instance) true)))))

(event OnComponentEndOverlap(Box)
  (params (OverlappedComponent :type Primitive%20Component%20Object%20Reference) (OtherActor :type Actor%20Object%20Reference) (OtherComp :type Primitive%20Component%20Object%20Reference) (OtherBodyIndex :type Integer))
  (bind _asbp_gomer_character (Utilities|Casting|CastToBP_GomerCharacter OtherActor))
  (Variables|/Game/GomerContent/Blueprints/BP_GameInstance.BP_GameInstance_C|SetbControlVisible (Variables|/Game/GomerContent/Blueprints/BP_GomerCharacter.BP_GomerCharacter_C|GetGame%20Instance _asbp_gomer_character) false)
  (if (and (Variables|/Game/GomerContent/Blueprints/BP_GameInstance.BP_GameInstance_C|GetbTalking (Variables|/Game/GomerContent/Blueprints/BP_GomerCharacter.BP_GomerCharacter_C|GetGame%20Instance _asbp_gomer_character)) (not (Variables|/Game/GomerContent/Blueprints/BP_GomerCharacter.BP_GomerCharacter_C|GetbBoxDone _asbp_gomer_character)))
    (Utilities|FlowControl|Delay 1.0)
    (UserInterface|Animation|PlayAnimation (Variables|/Game/GomerContent/Blueprints/BP_GomerCharacter.BP_GomerCharacter_C|GetNPC%20Dialogue%20Reference _asbp_gomer_character) (Variables|/Game/GomerContent/UMG/NPC_Dialogue.NPC_Dialogue_C|GetTalkEnd (Variables|/Game/GomerContent/Blueprints/BP_GomerCharacter.BP_GomerCharacter_C|GetNPC%20Dialogue%20Reference _asbp_gomer_character)) 0.0 1 "Forward" 1.0)
    (Variables|/Game/GomerContent/UMG/NPC_Dialogue.NPC_Dialogue_C|SetString%20Index (Variables|/Game/GomerContent/Blueprints/BP_GomerCharacter.BP_GomerCharacter_C|GetNPC%20Dialogue%20Reference _asbp_gomer_character) 0)
    (Variables|/Game/GomerContent/UMG/NPC_Dialogue.NPC_Dialogue_C|SetPrint%20String (Variables|/Game/GomerContent/Blueprints/BP_GomerCharacter.BP_GomerCharacter_C|GetNPC%20Dialogue%20Reference _asbp_gomer_character) "")
    (Utilities|Array|Clear (Variables|/Game/GomerContent/UMG/NPC_Dialogue.NPC_Dialogue_C|GetString%20Array (Variables|/Game/GomerContent/Blueprints/BP_GomerCharacter.BP_GomerCharacter_C|GetNPC%20Dialogue%20Reference _asbp_gomer_character)))
    (Variables|/Game/GomerContent/Blueprints/BP_GomerCharacter.BP_GomerCharacter_C|SetDialogue%20Count _asbp_gomer_character -1)))

(event EventBeginPlay
  (bind _asbp_game_instance (Utilities|Casting|CastToBP_GameInstance (Game|GetGameInstance)))
  (Variables|/Game/GomerContent/Blueprints/BP_GameInstance.BP_GameInstance_C|SetHubWorldNPC _asbp_game_instance self))

(fn ConstructionScript
  (|CallParentFunction))

(fn BounceDirection
  (params (Vector%20A :type Vector) (Vector%20B :type Vector))
  (return (Math|Vector|Normalize (- Vector%20A (* (* Vector%20B (Math|Vector|DotProduct Vector%20A Vector%20B)) 2.0)))))

(fn WallCheck
  (params (Normal :type Vector))
  (bind (_x _y) (Math|Vector|BreakVector Normal))
  (bind _returnvalue (Math|Float|Absolute(Float) _x))
  (bind _returnvalue_2 (Math|Float|Absolute(Float) _y))
  (bind _returnvalue_3 (+ _returnvalue _returnvalue_2))
  (Math|Float|CompareFloat _returnvalue_3 0.0
    (:>
      (Variables|Default|SetbCanDashAttack? (Math|Boolean|ANDBoolean (Utilities|Enum|Equal(Enum) (Variables|/Script/Engine.CharacterMovementComponent|GetMovementMode (Variables|Character|GetCharacterMovement)) "MOVE_Falling") (not (Math|Float|NearlyEqual(Float) _returnvalue_3 0.0 1e-06)) (Variables|Default|GetbIsDashing))))
    (:==
      (Variables|Default|SetbCanDashAttack? false)))
  (return (Variables|Default|GetbCanDashAttack?)))