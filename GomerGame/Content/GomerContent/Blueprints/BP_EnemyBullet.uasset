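; BP_EnemyBullet is an enemy projectile that drains Power from the player's Gomer character.
; BeginPlay casts the player character to BP_GomerCharacter and caches it with its GameInstance.
; Overlapping Gomer reduces Power on that GameInstance, and any overlap destroys the bullet except with the two intro enemy classes.
; A blocking hit destroys it without damage, ignoring only BP_IntroEnemy.
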(event EventBeginPlay
  (bind _asbp_gomer_character (Utilities|Casting|CastToBP_GomerCharacter (Game|GetPlayerCharacter 0)))
  (Variables|Default|SetGomer _asbp_gomer_character)
  (Variables|Default|SetGame%20Instance (Variables|/Game/GomerContent/Blueprints/BP_GomerCharacter.BP_GomerCharacter_C|GetGame%20Instance _asbp_gomer_character)))

(event Collision|EventActorBeginOverlap
  (params (OtherActor :type Actor%20Object%20Reference))
  (if (not (or (== (Utilities|GetClass OtherActor) "/Game/GomerContent/Blueprints/BP_IntroEnemy.BP_IntroEnemy_C") (== (Utilities|GetClass OtherActor) "/Game/GomerContent/Blueprints/BP_IntroEnemyInterp.BP_IntroEnemyInterp_C")))
    (if (== (Utilities|GetClass OtherActor) "/Game/GomerContent/Blueprints/BP_GomerCharacter.BP_GomerCharacter_C")
      (Variables|/Game/GomerContent/Blueprints/BP_GameInstance.BP_GameInstance_C|SetPower (Variables|/Game/GomerContent/Blueprints/BP_GomerCharacter.BP_GomerCharacter_C|GetGame%20Instance (stale EventBeginPlay _asbp_gomer_character)) (- (Variables|/Game/GomerContent/Blueprints/BP_GameInstance.BP_GameInstance_C|GetPower (Variables|/Game/GomerContent/Blueprints/BP_GomerCharacter.BP_GomerCharacter_C|GetGame%20Instance (stale EventBeginPlay _asbp_gomer_character))) 0.2)))
    (Actor|DestroyActor)))

(event EventTick
  (params (DeltaSeconds :type Float%20%28single-precision%29)))

(event Collision|EventHit
  (params (MyComp :type Primitive%20Component%20Object%20Reference) (Other :type Actor%20Object%20Reference) (OtherComp :type Primitive%20Component%20Object%20Reference) (bSelfMoved :type Boolean) (HitLocation :type Vector :default "0, 0, 0") (HitNormal :type Vector :default "0, 0, 0") (NormalImpulse :type Vector :default "0, 0, 0") (Hit :type Hit%20Result%20Structure%20%28by%20ref%29))
  (if (not (== (Utilities|GetClass Other) "/Game/GomerContent/Blueprints/BP_IntroEnemy.BP_IntroEnemy_C"))
    (Actor|DestroyActor)))

(fn ConstructionScript)