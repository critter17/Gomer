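; Gomer, the player character, with an air dash, an upward spin, NPC dialogue, pause menu, checkpoints and game over at zero Power.
; Dashes into walls reflect off the hit normal into a bounce.
; Dash, bounce and spin share a retriggerable delay that restores movement; landing refills charges, which live in the GameInstance.
; A DialogueCount state machine drives the NPC conversation that trades five nuts for the spin upgrade.
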(event EventOnLanded
  (params (Hit :type Hit%20Result%20Structure%20%28by%20ref%29))
  (bind _charactermovement (Variables|Character|GetCharacterMovement))
  (bind _game_instance (Variables|Default|GetGame%20Instance))
  (if (not (== (Utilities|GetClass (.HitActor (Collision|BreakHitResult Hit))) "/Game/GomerContent/Blueprints/BP_IntroEnemy.BP_IntroEnemy_C"))
    ;[1 1 1] Landing Refresh (Dashes and player control
    (Variables|/Game/GomerContent/Blueprints/BP_GameInstance.BP_GameInstance_C|SetNumDashes _game_instance 1)
    (Variables|/Game/GomerContent/Blueprints/BP_GameInstance.BP_GameInstance_C|SetNumSpins _game_instance 1)
    (Variables|Default|SetbIsDashing false)
    (Variables|Default|SetbIsSpinning false)
    (Variables|Default|SetbCanDashAttack? false)
    (Components|Capsule|SetCapsuleSize (Variables|Default|GetCapsuleComponent) 2e+01 55.0 true)
    (Variables|/Script/Engine.CharacterMovementComponent|SetbIgnoreBaseRotation _charactermovement false)
    (Input|ResetIgnoreMoveInput (Pawn|GetController))
    (Variables|/Script/Engine.CharacterMovementComponent|SetGravityScale _charactermovement 4.0)))

(event EventTick
  (params (DeltaSeconds :type Float%20%28single-precision%29))
  (if (Math|Float|NearlyEqual(Float) (Variables|/Game/GomerContent/Blueprints/BP_GameInstance.BP_GameInstance_C|GetPower (Variables|Default|GetGame%20Instance)) 0.0 1e-06)
    (bind _returnvalue (Game|GetCurrentLevelName true))
    (Variables|/Game/GomerContent/Blueprints/BP_GameInstance.BP_GameInstance_C|SetLevel%20Name (Variables|Default|GetGame%20Instance) _returnvalue)
    (Actor|DestroyActor)
    (Game|OpenLevel(byName) "GameOver")))

(event EventBeginPlay
  (bind _returnvalue (UserInterface|CreateWidget "/Game/GomerContent/UMG/PauseMenu.PauseMenu_C"))
  (Variables|Default|SetPause%20Menu _returnvalue)
  (bind _returnvalue_2 (UserInterface|CreateWidget "/Game/GomerContent/UMG/NPC_Dialogue.NPC_Dialogue_C"))
  (Variables|Default|SetNPC%20Dialogue%20Reference _returnvalue_2)
  (bind _asbp_game_instance (Utilities|Casting|CastToBP_GameInstance (Game|GetGameInstance)))
  (Variables|Default|SetGame%20Instance _asbp_game_instance)
  (bind _returnvalue_3 (UserInterface|CreateWidget "/Game/GomerContent/UMG/UIHUD.UIHUD_C"))
  (bind _output_get (Variables|Default|SetHUD%20Reference _returnvalue_3))
  (UserInterface|Viewport|AddtoViewport _output_get 0)
  (Variables|/Game/GomerContent/Blueprints/BP_GameInstance.BP_GameInstance_C|SetPlayer%20Spawn%20Location (Variables|Default|GetGame%20Instance) (Transformation|GetActorLocation))
  (Variables|/Game/GomerContent/Blueprints/BP_GameInstance.BP_GameInstance_C|SetPlayer%20Spawn%20Rotation (Variables|Default|GetGame%20Instance) (Transformation|GetActorRotation))
  (Input|SetInputModeGameOnly (Game|GetPlayerController 0)))

(event Collision|EventActorBeginOverlap
  (params (OtherActor :type Actor%20Object%20Reference))
  (bind _game_instance (Variables|Default|GetGame%20Instance))
  (if (not (== (Utilities|GetClass OtherActor) "/Game/GomerContent/Blueprints/gear_Blueprint.gear_Blueprint_C"))
    (if (== (Utilities|GetClass OtherActor) "/Game/GomerContent/Blueprints/BP_RespawnPoint.BP_RespawnPoint_C")
      (bind _asbp_respawn_point (Utilities|Casting|CastToBP_RespawnPoint OtherActor))
      (Variables|/Game/GomerContent/Blueprints/BP_GameInstance.BP_GameInstance_C|SetPlayer%20Spawn%20Location _game_instance (Variables|/Game/GomerContent/Blueprints/BP_RespawnPoint.BP_RespawnPoint_C|GetRespawn%20Box%20Location _asbp_respawn_point))
      (Variables|/Game/GomerContent/Blueprints/BP_GameInstance.BP_GameInstance_C|SetPlayer%20Spawn%20Rotation _game_instance (Transformation|GetActorRotation)))))

(event Collision|EventHit
  (params (MyComp :type Primitive%20Component%20Object%20Reference) (Other :type Actor%20Object%20Reference) (OtherComp :type Primitive%20Component%20Object%20Reference) (bSelfMoved :type Boolean) (HitLocation :type Vector :default "0, 0, 0") (HitNormal :type Vector) (NormalImpulse :type Vector :default "0, 0, 0") (Hit :type Hit%20Result%20Structure%20%28by%20ref%29))
  (bind _charactermovement (Variables|Character|GetCharacterMovement))
  (bind _charactermovement_2 (Variables|Character|GetCharacterMovement))
  (bind _valid_wall (CallFunction|WallCheck HitNormal))
  (if _valid_wall
    (bind _output_get (Variables|Default|SetForwardV (Transformation|GetActorForwardVector (Class|CharacterMovementComponent|GetCharacterOwner (Variables|Character|GetCharacterMovement)))))
    (bind _output_get_2 (Variables|Default|SetNormalV HitNormal))
    (bind _r (CallFunction|BounceDirection _output_get _output_get_2))
    (Variables|Default|SetGomer%20Velocity (* _r 1e+03))
    (Variables|Default|SetGomerRotation (Math|Conversions|RotationFromXVector (* _r 1e+03)))
    (Components|Capsule|SetCapsuleSize (Variables|Default|GetCapsuleComponent) 4e+01 45.0 true)
    (Variables|/Script/Engine.CharacterMovementComponent|SetGravityScale _charactermovement_2 0.0)
    (Variables|/Script/Engine.CharacterMovementComponent|SetbIgnoreBaseRotation _charactermovement_2 true)
    (Input|SetIgnoreMoveInput (Pawn|GetController) true)
    (Character|LaunchCharacter (Variables|Default|GetGomer%20Velocity) true true)
    (Transformation|SetActorRotation (Variables|Default|GetGomerRotation))
    (Variables|Default|SetDashDelay 0.7)
    ;[1 1 1] Dash
    (Utilities|FlowControl|RetriggerableDelay (Variables|Default|GetDashDelay))
    ;[1 1 1] End of dash
    (Variables|Default|SetbIsDashing false)
    (Variables|Default|SetbIsSpinning false)
    (Variables|Default|SetbCanDashAttack? false)
    (Variables|/Script/Engine.CharacterMovementComponent|SetGravityScale _charactermovement 4.0)
    (Components|Capsule|SetCapsuleSize (Variables|Default|GetCapsuleComponent) 2e+01 55.0 true)
    (Variables|/Script/Engine.MovementComponent|SetVelocity _charactermovement "0, 0, 0")
    (Variables|/Script/Engine.CharacterMovementComponent|SetbIgnoreBaseRotation _charactermovement false)
    (Input|ResetIgnoreMoveInput (Pawn|GetController))))

(event Input|ActionEvents|InputActionInteract
  (params (Key :type Key%20Structure :default "AnyKey"))
  (bind _game_instance (Variables|Default|GetGame%20Instance))
  (bind _numnuts (Variables|/Game/GomerContent/Blueprints/BP_GameInstance.BP_GameInstance_C|GetNumNuts _game_instance))
  (:Pressed
    (if (and (not (Variables|/Game/GomerContent/Blueprints/BP_GameInstance.BP_GameInstance_C|GetbTalking _game_instance)) (Variables|/Game/GomerContent/Blueprints/BP_GameInstance.BP_GameInstance_C|GetbControlVisible _game_instance))
      (Variables|/Game/GomerContent/Blueprints/BP_GameInstance.BP_GameInstance_C|SetbTalking _game_instance true)
      (if (Variables|Default|GetbExVis)
        (Variables|Default|SetDialogue%20Count 3)
        (CallFunction|SelectFirstDialogue :!label _label)
        (elif (== _numnuts 0)
          (Variables|Default|SetDialogue%20Count 0)
          (goto _label)
          (elif (>= _numnuts 5)
            (Variables|Default|SetDialogue%20Count 1)
            (goto _label)
            (elif (not (== (Variables|Default|GetDialogue%20Count) 4))
              (Variables|Default|SetDialogue%20Count 2)
              (goto _label))))))))

(event Input|ActionEvents|InputActionTalkContinue
  (params (Key :type Key%20Structure :default "AnyKey"))
  (bind _npc_dialogue_reference (Variables|Default|GetNPC%20Dialogue%20Reference))
  (bind _game_instance (Variables|Default|GetGame%20Instance))
  (:Pressed
    (switch int (Variables|Default|GetDialogue%20Count)
      (:0
        (UserInterface|Animation|PlayAnimation _npc_dialogue_reference (Variables|/Game/GomerContent/UMG/NPC_Dialogue.NPC_Dialogue_C|GetTalkEnd _npc_dialogue_reference) 0.0 1 "Forward" 1.0 :!label _label)
        (Variables|/Game/GomerContent/UMG/NPC_Dialogue.NPC_Dialogue_C|SetString%20Index _npc_dialogue_reference 0)
        (Variables|/Game/GomerContent/UMG/NPC_Dialogue.NPC_Dialogue_C|SetPrint%20String _npc_dialogue_reference "")
        (Utilities|Array|Clear (Variables|/Game/GomerContent/UMG/NPC_Dialogue.NPC_Dialogue_C|GetString%20Array _npc_dialogue_reference))
        (Variables|Default|SetDialogue%20Count -1)
        (Variables|Default|SetbBoxDone true))
      (:1
        (Variables|/Game/GomerContent/UMG/NPC_Dialogue.NPC_Dialogue_C|SetNPC%20Dialogue _npc_dialogue_reference (Variables|/Game/GomerContent/UMG/NPC_Dialogue.NPC_Dialogue_C|GetGot%20Upgrade _npc_dialogue_reference))
        (Variables|/Game/GomerContent/UMG/NPC_Dialogue.NPC_Dialogue_C|SetString%20Index _npc_dialogue_reference 0)
        (Variables|/Game/GomerContent/UMG/NPC_Dialogue.NPC_Dialogue_C|SetPrint%20String _npc_dialogue_reference "")
        (Utilities|Array|Clear (Variables|/Game/GomerContent/UMG/NPC_Dialogue.NPC_Dialogue_C|GetString%20Array _npc_dialogue_reference))
        (Variables|Default|SetDialogue%20Count 4)
        (Default|CustomEvent0 _npc_dialogue_reference))
      (:2
        (goto _label))
      (:3
        (goto _label))
      (:4
        (Variables|/Game/GomerContent/Blueprints/BP_GameInstance.BP_GameInstance_C|SetbSpinVisibility _game_instance true)
        (Rendering|SetVisibility (Actor|GetComponentbyClass (Variables|/Game/GomerContent/Blueprints/BP_GameInstance.BP_GameInstance_C|GetHubWorldNPC _game_instance) "/Script/Engine.TextRenderComponent") false false)
        (Variables|/Game/GomerContent/Blueprints/BP_GameInstance.BP_GameInstance_C|SetNumNuts _game_instance (- (Variables|/Game/GomerContent/Blueprints/BP_GameInstance.BP_GameInstance_C|GetNumNuts _game_instance) 5))
        (Variables|Default|SetbExVis true)
        (goto _label)))))

(event Input|ActionEvents|InputActionDash
  (params (Key :type Key%20Structure :default "AnyKey"))
  (bind _charactermovement (Variables|Character|GetCharacterMovement))
  (bind _charactermovement_2 (Variables|Character|GetCharacterMovement))
  (bind _game_instance (Variables|Default|GetGame%20Instance))
  (:Pressed
    (if (Math|Boolean|ANDBoolean (Utilities|Enum|Equal(Enum) (Variables|/Script/Engine.CharacterMovementComponent|GetMovementMode (Variables|Character|GetCharacterMovement)) "MOVE_Falling") (> (Variables|/Game/GomerContent/Blueprints/BP_GameInstance.BP_GameInstance_C|GetNumDashes (Variables|Default|GetGame%20Instance)) 0) (not (Variables|Default|GetbIsDashing)) (not (Variables|Default|GetbIsSpinning)))
      (Variables|Default|SetbIsDashing true)
      (if (not (Variables|Default|GetbCanDashAttack?))
        (Components|Capsule|SetCapsuleSize (Variables|Default|GetCapsuleComponent) 4e+01 45.0 true)
        (bind _output_get (Variables|Default|SetForwardV (Transformation|GetActorForwardVector (Class|CharacterMovementComponent|GetCharacterOwner (Variables|Character|GetCharacterMovement)))))
        (Variables|/Game/GomerContent/Blueprints/BP_GameInstance.BP_GameInstance_C|SetNumDashes _game_instance (- (Variables|/Game/GomerContent/Blueprints/BP_GameInstance.BP_GameInstance_C|GetNumDashes _game_instance) 1))
        (Variables|Default|SetGomer%20Velocity (* _output_get 6e+02))
        (Variables|/Script/Engine.CharacterMovementComponent|SetGravityScale _charactermovement 0.0)
        (if (Class|PawnMovementComponent|IsMoveInputIgnored _charactermovement)
          _
          (else
            (Variables|/Script/Engine.CharacterMovementComponent|SetbIgnoreBaseRotation _charactermovement true)))
        (Input|SetIgnoreMoveInput (Pawn|GetController) true)
        ;[1 1 1] Dash
        (Character|LaunchCharacter (Variables|Default|GetGomer%20Velocity) true true)
        (Variables|Default|SetDashDelay 1.019048)
        (Utilities|FlowControl|RetriggerableDelay (Variables|Default|GetDashDelay))
        ;[1 1 1] End of dash
        (Variables|Default|SetbIsDashing false)
        (Variables|Default|SetbIsSpinning false)
        (Variables|Default|SetbCanDashAttack? false)
        (Variables|/Script/Engine.CharacterMovementComponent|SetGravityScale _charactermovement_2 4.0)
        (Components|Capsule|SetCapsuleSize (Variables|Default|GetCapsuleComponent) 2e+01 55.0 true)
        (Variables|/Script/Engine.MovementComponent|SetVelocity _charactermovement_2 "0, 0, 0")
        (Variables|/Script/Engine.CharacterMovementComponent|SetbIgnoreBaseRotation _charactermovement_2 false)
        (Input|ResetIgnoreMoveInput (Pawn|GetController))))))

(event Input|ActionEvents|InputActionSpin
  (params (Key :type Key%20Structure :default "AnyKey"))
  (bind _charactermovement (Variables|Character|GetCharacterMovement))
  (bind _game_instance (Variables|Default|GetGame%20Instance))
  (bind _game_instance_2 (Variables|Default|GetGame%20Instance))
  (:Pressed
    (if (Math|Boolean|ANDBoolean (Utilities|Enum|Equal(Enum) (Variables|/Script/Engine.CharacterMovementComponent|GetMovementMode (Variables|Character|GetCharacterMovement)) "MOVE_Falling") (> (Variables|/Game/GomerContent/Blueprints/BP_GameInstance.BP_GameInstance_C|GetNumSpins _game_instance) 0) (not (Variables|Default|GetbIsSpinning)) (not (Variables|Default|GetbIsDashing)) (not (Variables|Default|GetbCanDashAttack?)) (Variables|/Game/GomerContent/Blueprints/BP_GameInstance.BP_GameInstance_C|GetbSpinVisibility _game_instance))
      (Variables|Default|SetbIsSpinning true)
      (Variables|/Game/GomerContent/Blueprints/BP_GameInstance.BP_GameInstance_C|SetNumSpins _game_instance_2 (- (Variables|/Game/GomerContent/Blueprints/BP_GameInstance.BP_GameInstance_C|GetNumSpins _game_instance_2) 1))
      (Variables|Default|SetGomer%20Velocity "0, 0,700.000000")
      (Variables|/Script/Engine.CharacterMovementComponent|SetbIgnoreBaseRotation (Variables|Character|GetCharacterMovement) true)
      (Input|SetIgnoreMoveInput (Pawn|GetController) true)
      (Character|LaunchCharacter (Variables|Default|GetGomer%20Velocity) true true)
      (Variables|Default|SetDashDelay 0.733333)
      ;[1 1 1] Dash
      (Utilities|FlowControl|RetriggerableDelay (Variables|Default|GetDashDelay))
      ;[1 1 1] End of dash
      (Variables|Default|SetbIsDashing false)
      (Variables|Default|SetbIsSpinning false)
      (Variables|Default|SetbCanDashAttack? false)
      (Variables|/Script/Engine.CharacterMovementComponent|SetGravityScale _charactermovement 4.0)
      (Components|Capsule|SetCapsuleSize (Variables|Default|GetCapsuleComponent) 2e+01 55.0 true)
      (Variables|/Script/Engine.MovementComponent|SetVelocity _charactermovement "0, 0, 0")
      (Variables|/Script/Engine.CharacterMovementComponent|SetbIgnoreBaseRotation _charactermovement false)
      (Input|ResetIgnoreMoveInput (Pawn|GetController)))))

(event Input|ActionEvents|InputActionPause
  (params (Key :type Key%20Structure :default "AnyKey"))
  (bind _returnvalue (Game|GetPlayerController 0))
  (bind _hud_reference (Variables|Default|GetHUD%20Reference))
  (:Pressed
    (if (Variables|Default|GetbPaused)
      (Game|SetGamePaused false)
      (Variables|/Script/Engine.PlayerController|SetbShowMouseCursor _returnvalue false)
      (Widget|RemovefromParent (Variables|Default|GetPause%20Menu))
      (Variables|Default|SetbPaused false)
      (Class|UserWidget|StopAnimation _hud_reference (Variables|/Game/GomerContent/UMG/UIHUD.UIHUD_C|GetGearOrNutGet _hud_reference))
      (UserInterface|Animation|PlayAnimation _hud_reference (Variables|/Game/GomerContent/UMG/UIHUD.UIHUD_C|GetGearOrNutOut _hud_reference) 0.0 1 "Forward" 1.0)
      (Input|SetInputModeGameOnly (Game|GetPlayerController 0))
      (else
        (bind _returnvalue_2 (Game|SetGamePaused true))
        (Variables|/Script/Engine.PlayerController|SetbShowMouseCursor _returnvalue _returnvalue_2)
        (UserInterface|Viewport|AddtoViewport (Variables|Default|GetPause%20Menu) 0)
        (Variables|Default|SetbPaused true)
        (Input|SetInputModeGameandUI (Game|GetPlayerController 0) (Variables|Default|GetPause%20Menu) "DoNotLock" true)))))

(fn ConstructionScript
  (|CallParentFunction)
  (Variables|Default|SetGomer%20Transform (Transformation|GetActorTransform)))

(fn BounceDirection
  (params (Vector%20A :type Vector) (Vector%20B :type Vector))
  (return (Math|Vector|Normalize (- Vector%20A (* (* Vector%20B (Math|Vector|DotProduct Vector%20A Vector%20B)) 2.0)))))

(fn WallCheck
  (params (Normal :type Vector))
  (bind (_x _y) (Math|Vector|BreakVector Normal))
  (bind _returnvalue (Math|Float|Absolute(Float) _x))
  (bind _returnvalue_2 (Math|Float|Absolute(Float) _y))
  (bind _returnvalue_3 (+ _returnvalue _returnvalue_2))
  (Math|Float|CompareFloat _returnvalue_3 0.0
    (:>
      (Variables|Default|SetbCanDashAttack? (Math|Boolean|ANDBoolean (Utilities|Enum|Equal(Enum) (Variables|/Script/Engine.CharacterMovementComponent|GetMovementMode (Variables|Character|GetCharacterMovement)) "MOVE_Falling") (not (Math|Float|NearlyEqual(Float) _returnvalue_3 0.0 1e-06)) (Variables|Default|GetbIsDashing))))
    (:==
      (Variables|Default|SetbCanDashAttack? false)))
  (return (Variables|Default|GetbCanDashAttack?)))

(fn EnemyCheck
  (bind _returnvalue (Transformation|GetActorForwardVector))
  (bind _charactermovement (Variables|Character|GetCharacterMovement))
  (bind _returnvalue_2 (* _returnvalue -1e+03))
  (bind (_x _y _z) (Math|Vector|BreakVector _returnvalue_2))
  (if (Variables|Default|GetbCanDashAttack?)
    (Variables|/Script/Engine.MovementComponent|SetVelocity _charactermovement (Variables|Default|GetGomer%20Velocity) :!label _label)
    (elif (Variables|Default|GetbIsSpinning)
      (goto _label)
      (else
        (Variables|/Script/Engine.CharacterMovementComponent|SetGravityScale _charactermovement 4e+01)
        (Character|LaunchCharacter (Math|Vector|MakeVector _x _y (+ _z 1e+03)) true true))))
  (return 0.5))

(fn GearCheck
  (if (Utilities|Enum|Equal(Enum) (Variables|/Script/Engine.CharacterMovementComponent|GetMovementMode (Variables|Character|GetCharacterMovement)) "MOVE_Walking")
    _
    (else
      _))
  (Variables|Default|SetGomer%20Velocity (Variables|/Script/Engine.MovementComponent|GetVelocity (Variables|Character|GetCharacterMovement))))

(fn FaceCamera
  (params (Gomer%20Rotation :type Rotator))
  (bind (_roll _pitch) (Math|Rotator|BreakRotator Gomer%20Rotation))
  (Transformation|SetActorRotation (Math|Rotator|MakeRotator _roll _pitch (.Yaw (Math|Rotator|BreakRotator (Math|Rotator|FindLookatRotation (Transformation|GetActorLocation) (Camera|GetCameraLocation (Variables|/Script/Engine.PlayerController|GetPlayerCameraManager (Game|GetPlayerController 0)))))))))

(fn SelectFirstDialogue
  (bind _npc_dialogue_reference (Variables|Default|GetNPC%20Dialogue%20Reference))
  (switch int (Variables|Default|GetDialogue%20Count)
    (:0
      (Variables|/Game/GomerContent/UMG/NPC_Dialogue.NPC_Dialogue_C|SetNPC%20Dialogue _npc_dialogue_reference (Variables|/Game/GomerContent/UMG/NPC_Dialogue.NPC_Dialogue_C|GetNo%20Nuts _npc_dialogue_reference)))
    (:1
      (Variables|/Game/GomerContent/UMG/NPC_Dialogue.NPC_Dialogue_C|SetNPC%20Dialogue _npc_dialogue_reference (Variables|/Game/GomerContent/UMG/NPC_Dialogue.NPC_Dialogue_C|GetEnough%20Nuts _npc_dialogue_reference)))
    (:2
      (Variables|/Game/GomerContent/UMG/NPC_Dialogue.NPC_Dialogue_C|SetNPC%20Dialogue _npc_dialogue_reference (Variables|/Game/GomerContent/UMG/NPC_Dialogue.NPC_Dialogue_C|GetFew%20Nuts _npc_dialogue_reference)))
    (:3
      (Variables|/Game/GomerContent/UMG/NPC_Dialogue.NPC_Dialogue_C|SetNPC%20Dialogue _npc_dialogue_reference (Variables|/Game/GomerContent/UMG/NPC_Dialogue.NPC_Dialogue_C|GetGot%20Upgrade _npc_dialogue_reference))))
  (UserInterface|Animation|PlayAnimation _npc_dialogue_reference (Variables|/Game/GomerContent/UMG/NPC_Dialogue.NPC_Dialogue_C|GetTalkBegin _npc_dialogue_reference) 0.0 1 "Forward" 1.0))