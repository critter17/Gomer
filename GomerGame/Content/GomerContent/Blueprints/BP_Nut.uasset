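; BP_Nut is a collectible nut pickup for the Gomer character.
; When its collision box overlaps BP_GomerCharacter, it increments the NumNuts count stored in BP_GameInstance and destroys itself.
; It plays a pickup sound at its location and triggers the character HUD's GearOrNutGet animation unless that animation is already playing.
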(event OnComponentBeginOverlap(CollisionBox)
  (params (OverlappedComponent :type Primitive%20Component%20Object%20Reference) (OtherActor :type Actor%20Object%20Reference) (OtherComp :type Primitive%20Component%20Object%20Reference) (OtherBodyIndex :type Integer) (bFromSweep :type Boolean) (SweepResult :type Hit%20Result%20Structure%20%28by%20ref%29))
  (if (== (Utilities|GetClass OtherActor) "/Game/GomerContent/Blueprints/BP_GomerCharacter.BP_GomerCharacter_C")
    (bind _asbp_gomer_character (Utilities|Casting|CastToBP_GomerCharacter OtherActor))
    (bind _asbp_game_instance (Utilities|Casting|CastToBP_GameInstance (Game|GetGameInstance)))
    (Variables|/Game/GomerContent/Blueprints/BP_GameInstance.BP_GameInstance_C|SetNumNuts _asbp_game_instance (+ (Variables|/Game/GomerContent/Blueprints/BP_GameInstance.BP_GameInstance_C|GetNumNuts _asbp_game_instance) 1))
    (Actor|DestroyActor)
    (Audio|PlaySoundatLocation "/Game/GomerContent/Sounds/Nut_Get_Cue.Nut_Get_Cue" (Transformation|GetActorLocation))
    (if (not (Class|UserWidget|IsAnimationPlaying (Variables|/Game/GomerContent/Blueprints/BP_GomerCharacter.BP_GomerCharacter_C|GetHUD%20Reference _asbp_gomer_character) (Variables|/Game/GomerContent/UMG/UIHUD.UIHUD_C|GetGearOrNutGet (Variables|/Game/GomerContent/Blueprints/BP_GomerCharacter.BP_GomerCharacter_C|GetHUD%20Reference _asbp_gomer_character))))
      (UserInterface|Animation|PlayAnimation (Variables|/Game/GomerContent/Blueprints/BP_GomerCharacter.BP_GomerCharacter_C|GetHUD%20Reference _asbp_gomer_character) (Variables|/Game/GomerContent/UMG/UIHUD.UIHUD_C|GetGearOrNutGet (Variables|/Game/GomerContent/Blueprints/BP_GomerCharacter.BP_GomerCharacter_C|GetHUD%20Reference _asbp_gomer_character)) 0.0 1 "Forward" 1.0))))

(event EventBeginPlay)

(event Collision|EventActorBeginOverlap
  (params (OtherActor :type Actor%20Object%20Reference)))

(event EventTick
  (params (DeltaSeconds :type Float%20%28single-precision%29)))

(fn ConstructionScript)