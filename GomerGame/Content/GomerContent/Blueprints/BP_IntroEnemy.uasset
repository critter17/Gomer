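; BP_IntroEnemy is a shooting enemy that fights the Gomer player character and respawns through the GameInstance when killed.
; Within range, Tick aims at Gomer and fires slightly spread BP_EnemyBullet projectiles after a random Delay.
; Dash or spin contact destroys it, tallies the move and saves its spawn transform for respawn.
; Other contact knocks Gomer back and drains Power, gated by a DoOnce with delayed reset.
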(event OnComponentBeginOverlap(CapsuleComponent)
  (params (OverlappedComponent :type Primitive%20Component%20Object%20Reference) (OtherActor :type Actor%20Object%20Reference) (OtherComp :type Primitive%20Component%20Object%20Reference) (OtherBodyIndex :type Integer) (bFromSweep :type Boolean) (SweepResult :type Hit%20Result%20Structure%20%28by%20ref%29))
  (bind _returnvalue (Transformation|GetActorForwardVector OtherActor))
  (bind _game_instance (Variables|Default|GetGame%20Instance))
  (bind _game_instance_2 (Variables|Default|GetGame%20Instance))
  (bind _game_instance_3 (Variables|Default|GetGame%20Instance))
  (bind _returnvalue_2 (* _returnvalue -1e+03))
  (bind (_x _y _z) (Math|Vector|BreakVector _returnvalue_2))
  (if (== (Utilities|GetClass OtherActor) "/Game/GomerContent/Blueprints/BP_GomerCharacter.BP_GomerCharacter_C")
    (bind _asbp_gomer_character (Utilities|Casting|CastToBP_GomerCharacter OtherActor))
    (if (Variables|/Game/GomerContent/Blueprints/BP_GomerCharacter.BP_GomerCharacter_C|GetbCanDashAttack? _asbp_gomer_character)
      (Variables|/Game/GomerContent/Blueprints/BP_GameInstance.BP_GameInstance_C|SetNumDashes _game_instance_3 (+ (Variables|/Game/GomerContent/Blueprints/BP_GameInstance.BP_GameInstance_C|GetNumDashes _game_instance_3) 1))
      (Variables|/Game/GomerContent/Blueprints/BP_GameInstance.BP_GameInstance_C|SetEnemy%20Spawn%20Transform _game_instance_2 (Variables|Default|GetLocal%20EST) :!label _label)
      (Actor|DestroyActor)
      (Default|RespawnEnemy _game_instance_2)
      (elif (Variables|/Game/GomerContent/Blueprints/BP_GomerCharacter.BP_GomerCharacter_C|GetbIsSpinning _asbp_gomer_character)
        (Variables|/Game/GomerContent/Blueprints/BP_GameInstance.BP_GameInstance_C|SetNumSpins _game_instance_3 (+ (Variables|/Game/GomerContent/Blueprints/BP_GameInstance.BP_GameInstance_C|GetNumSpins _game_instance_3) 1))
        (goto _label)
        (else
          (Utilities|FlowControl|DoOnce false :!label _label_2
            (:Completed
              (Variables|/Script/Engine.CharacterMovementComponent|SetGravityScale (Variables|/Script/Engine.Character|GetCharacterMovement _asbp_gomer_character) 4e+01)
              (Character|LaunchCharacter _asbp_gomer_character (Math|Vector|MakeVector _x _y (+ _z 8e+02)) true true)
              (Variables|/Game/GomerContent/Blueprints/BP_GameInstance.BP_GameInstance_C|SetPower _game_instance (- (Variables|/Game/GomerContent/Blueprints/BP_GameInstance.BP_GameInstance_C|GetPower _game_instance) 0.1))
              (Utilities|FlowControl|Delay 2.0)
              (if (or (Utilities|Enum|Equal(Enum) (Variables|/Script/Engine.CharacterMovementComponent|GetMovementMode (Variables|/Script/Engine.Character|GetCharacterMovement _asbp_gomer_character)) "MOVE_Walking") (Utilities|Enum|Equal(Enum) (Variables|/Script/Engine.CharacterMovementComponent|GetMovementMode (Variables|/Script/Engine.Character|GetCharacterMovement _asbp_gomer_character)) "MOVE_Falling"))
                (goto _label_2 Reset)))))))))

(event EventBeginPlay
  (bind _asbp_gomer_character (Utilities|Casting|CastToBP_GomerCharacter (Game|Player|GetPlayerPawn 0)))
  (bind _output_get (Variables|Default|SetGame%20Instance (Variables|/Game/GomerContent/Blueprints/BP_GomerCharacter.BP_GomerCharacter_C|GetGame%20Instance _asbp_gomer_character)))
  (Variables|/Game/GomerContent/Blueprints/BP_GameInstance.BP_GameInstance_C|SetGomer _output_get _asbp_gomer_character)
  (Variables|Default|SetLocal%20EST (Transformation|GetActorTransform)))

(event EventTick
  (params (DeltaSeconds :type Float%20%28single-precision%29))
  (bind _game_instance (Variables|Default|GetGame%20Instance))
  (bind _gomer (Variables|/Game/GomerContent/Blueprints/BP_GameInstance.BP_GameInstance_C|GetGomer _game_instance))
  (if (<= (Transformation|GetDistanceTo _gomer) 8e+02)
    (Utilities|IsValid _gomer
      (:Is%20Valid
        (Variables|Default|SetBullet%20Rotation (Math|Rotator|FindLookatRotation (Transformation|GetActorLocation) (Transformation|GetActorLocation _gomer)))
        (Utilities|FlowControl|Delay (Math|Random|RandomFloatinRange 3.0 6.0))
        (CallFunction|FireProjectile)))))

(fn ConstructionScript)

(fn FireProjectile
  (bind _returnvalue (Transformation|GetActorLocation))
  (bind _bullet_rotation (Variables|Default|GetBullet%20Rotation))
  (bind (_roll _pitch _yaw) (Math|Rotator|BreakRotator _bullet_rotation))
  (Game|SpawnActorfromClass "/Game/GomerContent/Blueprints/BP_EnemyBullet.BP_EnemyBullet_C" (Math|Transform|MakeTransform (+ _returnvalue (* (Math|Vector|GetForwardVector (Transformation|GetActorRotation)) 5e+01)) (Math|Rotator|MakeRotator _roll _pitch (+ _yaw (Math|Random|RandomFloatinRange -4.0 4.0)))) "AlwaysSpawn" 0 0)
  (Audio|PlaySoundatLocation "/Game/GomerContent/Sounds/Shoot_Cue.Shoot_Cue" _returnvalue))